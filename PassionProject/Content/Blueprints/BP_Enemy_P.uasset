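; BP_Enemy_P is an enemy that walks toward the altar and dies when hit by a player projectile.
; On BeginPlay it finds the BP_Alter_A actor, stores it as its target and moves to it with AI MoveTo.
; A collider hit by a first-person projectile destroys the projectile, increments the game mode's kill count, then destroys the enemy.
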(event `self.ReceiveBeginPlay`
  ; Move Enemy
  (bind _returnvalue (`GameplayStatics.GetActorOfClass` "/Game/Blueprints/BP_Alter_A.BP_Alter_A_C"))
  (set `self.alter target` _returnvalue)
  (`|AIMoveTo` self (0.0 0.0 0.0) (`self.alter target`) 2.0))

(event `self.collider.OnComponentHit`
  (params (HitComponent :type "PrimitiveComponent Object Reference") (OtherActor :type "Actor Object Reference") (OtherComp :type "PrimitiveComponent Object Reference") (NormalImpulse :type "Vector Structure") (Hit :type "HitResult Structure (by ref)"))
  (bind _asbp_first_person_projectile (cast `/Game/FirstPerson/Blueprints/BP_FirstPersonProjectile` OtherActor))
  (`self.K2_DestroyActor` _asbp_first_person_projectile)
  (bind _asbp_first_person_game_mode (cast `/Game/FirstPerson/Blueprints/BP_FirstPersonGameMode` (`GameplayStatics.GetGameMode`)))
  (`/Game/FirstPerson/Blueprints/BP_FirstPersonGameMode.incKills` _asbp_first_person_game_mode)
  (`self.K2_DestroyActor` self))

(fn `UserConstructionScript`)